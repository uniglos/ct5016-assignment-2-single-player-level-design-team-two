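; BP_BowPickup is a world pickup that gives the player the bow and reserve ammo for it.
; When BP_Player overlaps its PickupTrigger, it adds BowPickupAmmo to the player's bow reserve, sets HasBow and makes the player's Bow component visible.
; It then plays the Rifle_AmmoPickup sound at its location and destroys itself.
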(event `self.PickupTrigger.OnComponentBeginOverlap`
  (params (OverlappedComponent :type "PrimitiveComponent Object Reference") (OtherActor :type "Actor Object Reference") (OtherComp :type "PrimitiveComponent Object Reference") (OtherBodyIndex :type Integer) (bFromSweep :type Boolean) (SweepResult :type "HitResult Structure (by ref)"))
  (bind _asbp_player (cast `/Game/Blueprints/BP_Player` OtherActor))
  (set `/Game/Blueprints/BP_Player.BowReserveAmmo` (+ (`/Game/Blueprints/BP_Player.BowReserveAmmo` _asbp_player) (`self.BowPickupAmmo`)) _asbp_player)
  (set `/Game/Blueprints/BP_Player.hasBow` true _asbp_player)
  (`GameplayStatics.PlaySoundAtLocation` "/Game/PrototypeWeap/Sound/Rifle/Rifle_AmmoPickup.Rifle_AmmoPickup" (`self.K2_GetActorLocation`) (struct) 1.0 1.0 0.0 null null null null)
  (`SceneComponent.SetVisibility` (`/Game/Blueprints/BP_Player.Bow` _asbp_player) true false)
  (`self.K2_DestroyActor`))

(fn `UserConstructionScript`)